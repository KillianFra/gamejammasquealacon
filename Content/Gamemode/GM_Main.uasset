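; Main game mode that runs a monster-finding level among NPCs, mirroring counts to the game state.
; BeginPlay spawns a BP_NPC at every shuffled spawn point, each randomly a monster by MonsterRatio, independently of the computed totals.
; Interactions credit found monsters or deduct player health for wrong picks in the player state.
; Win/lose checks only print TODOs; the win check reads TotalMonsters, which interactions never decrement.
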(event `self.ReceiveBeginPlay`
  (set `self.CurrentLevel` 1)
  (`self.SpawnLevelNPCs`)
  (bind _asbp_game_state_main (cast `/Game/GameState/BP_GameState_Main` (`GameplayStatics.GetGameState`)))
  (set `self.GameStateRef` _asbp_game_state_main)
  (set `/Game/GameState/BP_GameState_Main.RemainingMonsters` (`self.RemainingMonsters`) _asbp_game_state_main)
  (set `/Game/GameState/BP_GameState_Main.RemainingNPCs` (`self.RemainingNPCs`) _asbp_game_state_main)
  (set `/Game/GameState/BP_GameState_Main.CurrentLevel` (`self.CurrentLevel`) _asbp_game_state_main))

(event `/Game/Interface/BPI_Interactable.OnNPCInteracted`
  (params (Interactor :type "/Game/clement_character/BP_Player Object Reference") (isMonster :type Boolean))
  (bind _playerstate (`self.PlayerState`))
  (bind _gamestateref (`self.GameStateRef`))
  (bind _playerstate_2 (`self.PlayerState`))
  (bind _playerstate_3 (`self.PlayerState`))
  (bind _asbp_player_state_main (cast `/Game/PlayerState/BP_PlayerState_Main` (`Controller.PlayerState` (`GameplayStatics.GetPlayerController` 0))))
  (set `self.PlayerState` _asbp_player_state_main)
  (if isMonster
    (set `/Game/PlayerState/BP_PlayerState_Main.MonstersFound` (+ (`/Game/PlayerState/BP_PlayerState_Main.MonstersFound` _playerstate_3) 1) _playerstate_3)
    (set `self.RemainingMonsters` (- (`self.RemainingMonsters`) 1))
    (set `self.RemainingNPCs` (- (`self.RemainingNPCs`) 1))
    (else
      (set `/Game/PlayerState/BP_PlayerState_Main.Health` (- (`/Game/PlayerState/BP_PlayerState_Main.Health` _playerstate) 1) _playerstate)
      (set `/Game/PlayerState/BP_PlayerState_Main.WrongChoices` (+ (`/Game/PlayerState/BP_PlayerState_Main.WrongChoices` _playerstate_2) 1) _playerstate_2)
      (set `self.RemainingNPCs` (- (`self.RemainingNPCs`) 1))))
  (set `/Game/GameState/BP_GameState_Main.RemainingNPCs` (`self.RemainingNPCs`) _gamestateref)
  (set `/Game/GameState/BP_GameState_Main.RemainingMonsters` (`self.RemainingMonsters`) _gamestateref)
  (`self.CheckLoseCondition`)
  (`self.CheckWinCondition`))

(fn `CheckLoseCondition`
  (bind _asbp_player_state_main (cast `/Game/PlayerState/BP_PlayerState_Main` (`Controller.PlayerState` (`GameplayStatics.GetPlayerController` 0))))
  (if (<= (`/Game/PlayerState/BP_PlayerState_Main.Health` _asbp_player_state_main) 0)
    (`KismetSystemLibrary.PrintString` "TODO: TRIGGER THE GAME OVER MENU")))

(fn `CheckWinCondition`
  (if (<= (`self.TotalMonsters`) 0)
    (`KismetSystemLibrary.PrintString` "TODO: Level complete function")))

(fn `SpawnLevelNPCs`
  (locals (SpawnPointList :type "Array of /Game/Utils/BP_SpawnPointNPC Object Reference") (CurrentSpawnPoint :type "/Game/Utils/BP_SpawnPointNPC Object Reference"))
  (bind _returnvalue (`self.GetTransform` (`local.CurrentSpawnPoint`)))
  (bind _outactors (`GameplayStatics.GetAllActorsOfClass` "/Game/Utils/BP_SpawnPointNPC.BP_SpawnPointNPC_C"))
  (bind _output_get (set `local.SpawnPointList` _outactors))
  (`KismetArrayLibrary.Array_Shuffle` _output_get)
  (bind _output_get_2 (set `self.TotalNPCs` (`self.NPCsPerLevel`)))
  (set `self.RemainingNPCs` _output_get_2)
  (bind _output_get_3 (set `self.TotalMonsters` (`KismetMathLibrary.Round` (* (`self.NPCsPerLevel`) (`self.MonsterRatio`)))))
  (set `self.RemainingMonsters` _output_get_3)
  (for _array_element (`local.SpawnPointList`)
    (set `local.CurrentSpawnPoint` _array_element)
    (if (> 0 (`self.NPCsPerLevel`))
      (break)
      (elif (< (`KismetMathLibrary.RandomFloat`) (`self.MonsterRatio`))
        (`|SpawnActorFromClass` "/Game/Characters/BP_NPC.BP_NPC_C" _returnvalue "Undefined" "MultiplyWithRoot" null true null)
        (else
          (`|SpawnActorFromClass` "/Game/Characters/BP_NPC.BP_NPC_C" _returnvalue "Undefined" "MultiplyWithRoot" null false null))))))

(fn `UserConstructionScript`)