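; BP_NPC is a human or monster NPC character that wanders, detects interactables and can be targeted by cursor.
; A looping, randomly offset timer asks BP_NPC_Controller for wander targets while no player is near.
; Its debug-drawn sphere maintains DetectList of BPI_Interactable actors, prompting the controller to evaluate the nearest.
; Hovering Circle when near sets the player's target; StopMovement halts it and notifies GM_Main, while PlayAnimation only swaps materials as a placeholder.
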(event `self.circle.OnBeginCursorOver`
  (params (TouchedComponent :type "PrimitiveComponent Object Reference"))
  (bind _asbp_player (cast `/Game/clement_character/BP_Player` (`GameplayStatics.GetPlayerCharacter` 0)))
  (if (`self.IsPlayerNear`)
    (set `/Game/clement_character/BP_Player.TargetedNPC` self _asbp_player)))

(event `self.ReceiveTick`
  (params (DeltaSeconds :type "Float (single-precision)"))
  (bind _sphere_collider (`self.Sphere_Collider`))
  ; Comment
  (`KismetSystemLibrary.DrawDebugSphere` (`SceneComponent.K2_GetComponentLocation` _sphere_collider) (`SphereComponent.SphereRadius` _sphere_collider) 12 (struct :`R` 1.0 :`G` 1.0 :`B` 1.0 :`A` 1.0) 0.1))

(event `self.ReceiveBeginPlay`
  (`SphereComponent.SetSphereRadius` (`self.Sphere_Collider`) (`self.DetectionRadius`) true)
  (`KismetSystemLibrary.K2_SetTimerDelegate` (delegate `WanderTick`) (+ (`self.WanderInterval`) (`KismetMathLibrary.RandomFloatInRange` -1.0 1.0)) true))

(event `WanderTick`
  (if (not (`self.IsPlayerNear`))
    (bind _asbp_npc_controller (cast `/Game/AI/BP_NPC_Controller` (`self.GetController`)))
    (`/Game/AI/BP_NPC_Controller.PickWanderTarget` _asbp_npc_controller)))

(event `self.Sphere_Collider.OnComponentBeginOverlap`
  (params (OverlappedComponent :type "PrimitiveComponent Object Reference") (OtherActor :type "Actor Object Reference") (OtherComp :type "PrimitiveComponent Object Reference") (OtherBodyIndex :type Integer) (bFromSweep :type Boolean) (SweepResult :type "HitResult Structure (by ref)"))
  (if (!= OtherActor self)
    (if (`KismetSystemLibrary.DoesImplementInterface` OtherActor "/Game/Interface/BPI_Interactable.BPI_Interactable_C")
      (`KismetArrayLibrary.Array_AddUnique` (`self.DetectList`) OtherActor)
      (bind _asbp_npc_controller (cast `/Game/AI/BP_NPC_Controller` (`self.GetController`))
        (:`then`
          (`/Game/AI/BP_NPC_Controller.EvaluateNearestTarget` _asbp_npc_controller))
        (:`CastFailed`
          (`KismetSystemLibrary.PrintString` "Hello"))))))

(event `self.Sphere_Collider.OnComponentEndOverlap`
  (params (OverlappedComponent :type "PrimitiveComponent Object Reference") (OtherActor :type "Actor Object Reference") (OtherComp :type "PrimitiveComponent Object Reference") (OtherBodyIndex :type Integer))
  (`KismetArrayLibrary.Array_RemoveItem` (`self.DetectList`) OtherActor))

(event `StopMovement`
  (set `self.State` "NewEnumerator2")
  (`KismetSystemLibrary.PrintString` "TODO: Play the fucking animation")
  (bind _asbp_npc_controller (cast `/Game/AI/BP_NPC_Controller` (`self.GetController`)))
  (`Controller.StopMovement` _asbp_npc_controller)
  (bind _asgm_main (cast `/Game/Gamemode/GM_Main` (`GameplayStatics.GetGameMode`)))
  (`/Game/Interface/BPI_Interactable.OnNPCInteracted` _asgm_main null (`self.IsMonster`)))

(fn `NewFunction`)

(fn `PlayAnimation`
  (returns (wasMonster :type Boolean))
  (bind _circle (`self.circle`))
  (if (`self.IsMonster`)
    (`KismetSystemLibrary.PrintString` "TODO: implement animation of monster")
    (`PrimitiveComponent.SetMaterial` _circle 0 "/Engine/VREditor/UI/ArrowMaterial.ArrowMaterial")
    (return true)
    (else
      (`KismetSystemLibrary.PrintString` "TODO: implement animation of Human")
      (`PrimitiveComponent.SetMaterial` _circle 0 "/Engine/VREditor/BasicMeshes/MI_Cube_03.MI_Cube_03")
      (return false))))

(fn `UserConstructionScript`)