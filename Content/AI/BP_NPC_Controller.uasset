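; AI controller for BP_NPC that switches it between random wandering and walking to detected interactibles, using the NPC's State enum.
; On possess it picks a reachable wander point; EvaluateNearestTarget, uncalled here, sends it to the closest DetectList actor via StartGoingTo.
; MoveCompleted would trigger animation and interaction or resume wandering, but its binding is disconnected.
; StartGoingTo is unfinished: it resets to wander once the move request succeeds, and CurrentTarget is never assigned.
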(event `self.ReceivePossess`
  (params (PossessedPawn :type "Pawn Object Reference"))
  (bind _asbp_npc (cast `/Game/Characters/BP_NPC` PossessedPawn))
  (set `self.PlayerRef` _asbp_npc)
  (`self.PickWanderTarget`))

(event `MoveCompleted` :!signature `self.ReceiveMoveCompleted`
  (params (RequestID :type "AIRequestID Structure") (Result :type "EPathFollowingResult Enum" :default "Success"))
  (if (select `EPathFollowingResult` Result :`Success` true)
    (bind _asbp_npc (cast `/Game/Characters/BP_NPC` (`self.K2_GetPawn`)))
    (if (`|EnumEquality` (`/Game/Characters/BP_NPC.State` _asbp_npc) "NewEnumerator1")
      (`self.HandleArrivedAtTarget`)
      (else
        (`self.ResumeWander`)))))

(fn `EvaluateNearestTarget`
  (locals (ClosestActor :type "Actor Object Reference") (ClosestDistance :type "Float (double-precision)" :default 9999999.0))
  (if (`KismetArrayLibrary.Array_IsEmpty` (`/Game/Characters/BP_NPC.DetectList` (`self.PlayerRef`)))
    (`self.ResumeWander`)
    (else
      (for _array_element (`/Game/Characters/BP_NPC.DetectList` (`self.PlayerRef`))
        (bind _returnvalue (`self.GetDistanceTo` _array_element (`self.PlayerRef`)))
        (if (< _returnvalue (`local.ClosestDistance`))
          (set `local.ClosestDistance` _returnvalue)
          (set `local.ClosestActor` _array_element)))
      (if (!= (`self.lastSeenTarget`) (`local.ClosestActor`))
        (`self.StartGoingTo` (`local.ClosestActor`))
        (else
          (set `/Game/Characters/BP_NPC.State` "NewEnumerator0" (`self.PlayerRef`)))))))

(fn `HandleArrivedAtTarget`
  (set `/Game/Characters/BP_NPC.State` "NewEnumerator2" (`self.PlayerRef`))
  (`/Game/Characters/BP_NPC.PlayAnimation` (`self.PlayerRef`))
  (message `/Game/Interface/BPI_Interactable.Interact` (`self.CurrentTarget`) (`self.PlayerRef`))
  (`self.ResumeWander`))

(fn `PickWanderTarget`
  (locals (NpcRef :type "/Game/Characters/BP_NPC Object Reference"))
  (if (`|EnumEquality` (`/Game/Characters/BP_NPC.State` (`self.PlayerRef`)) "NewEnumerator0")
    (`self.MoveToLocation` (`NavigationSystemV1.K2_GetRandomReachablePointInRadius` (`self.K2_GetActorLocation`) (`/Game/Characters/BP_NPC.WanderRadius` (`self.PlayerRef`)) null null) 10.0 true true false true null)))

(fn `ResumeWander`
  (set `/Game/Characters/BP_NPC.State` "NewEnumerator0" (`self.PlayerRef`))
  (`self.PickWanderTarget`))

(fn `StartGoingTo`
  (params (Target :type "Actor Object Reference"))
  (set `/Game/Characters/BP_NPC.State` "NewEnumerator1" (`self.PlayerRef`))
  (bind _returnvalue (`self.MoveToActor` Target 20.0 true true true null))
  (bind _asbp_generic_interactible (cast `/Game/Interactibles/BP_Generic_Interactible` Target))
  ; TODO: play the animation of the player
  (`KismetSystemLibrary.PrintString` (`|GetEnumeratorNameAsString` (`/Game/Interactibles/BP_Generic_Interactible.InteractibleType` _asbp_generic_interactible)))
  (switch `EPathFollowingRequestResult` _returnvalue
    (:`RequestSuccessful`
      (`KismetArrayLibrary.Array_RemoveItem` (`/Game/Characters/BP_NPC.DetectList` (`self.PlayerRef`)) Target)
      (set `/Game/Characters/BP_NPC.State` "NewEnumerator0" (`self.PlayerRef`)))))

(fn `UserConstructionScript`)